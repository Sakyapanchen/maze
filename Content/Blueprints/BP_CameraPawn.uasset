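; Orbit camera pawn for a maze scene that also lets the player drop balls and regenerate the maze.
; On start it possesses itself, shows the cursor and, given a valid maze, centers on it and scales spring arm length to its size.
; Mouse axes rotate the pawn with clamped pitch, and the wheel zooms.
; Tab spawns a falling ball above the cursor hit, while Space destroys tagged balls and regenerates the maze.
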(event `self.ReceiveBeginPlay`
  (`parent.ReceiveBeginPlay`)
  (`self.SetStartParams`))

(event `self.ReceiveTick`
  (params (DeltaSeconds :type "Float (single-precision)"))
  (`parent.ReceiveTick` DeltaSeconds)
  (`self.UpdatePitch`))

(event `Key|Tab`
  (params (Key :type "Key Structure"))
  ;[1 1 1] Spawn balls
  (:`Pressed`
    (`self.SpawnBall`)))

(event `Key|MouseScrollUp`
  (params (Key :type "Key Structure"))
  (bind _springarm (`self.SpringArm`))
  ;[1 1 1] Zoom
  (:`Pressed`
    (set `SpringArmComponent.TargetArmLength` (`KismetMathLibrary.FClamp` (- (`SpringArmComponent.TargetArmLength` _springarm) (`self.ZoomStep`)) (`self.MinArmLenght`) (`SpringArmComponent.TargetArmLength` (`self.SpringArm`))) _springarm)))

(event `Key|MouseScrollDown`
  (params (Key :type "Key Structure"))
  (bind _springarm (`self.SpringArm`))
  ;[1 1 1] Zoom
  (:`Pressed`
    (set `SpringArmComponent.TargetArmLength` (+ (`SpringArmComponent.TargetArmLength` _springarm) (`self.ZoomStep`)) _springarm)))

(event `Key|SpaceBar`
  (params (Key :type "Key Structure"))
  ;[1 1 1] Refresh
  (:`Pressed`
    (`self.RemoveBalls`)
    (bind _maze (`self.Maze`)
      (:`then`
        (`MazeGenerator.GenerateMaze` _maze))
      (:`else`))))

(event `UpdatePitch`
  (bind _pitchmin (`self.PitchMin`))
  (bind _pitchmax (`self.PitchMax`))
  (bind _pitch (.pitch (`self.K2_GetActorRotation`)))
  (bind _returnvalue (< _pitch _pitchmin))
  ;[1 1 1] Pitch limitation
  (if (or _returnvalue (> _pitch _pitchmax))
    (`self.K2_SetActorRotation` (`KismetMathLibrary.MakeRotator` 0.0 (`KismetMathLibrary.SelectFloat` _pitchmin _pitchmax _returnvalue) (.yaw (`self.K2_GetActorRotation`))) true)))

(event `InputAxisKey|MouseX`
  (params (AxisValue :type "Float (single-precision)"))
  ;[1 1 1] Look out
  (`self.K2_AddActorWorldRotation` (`KismetMathLibrary.MakeRotator` 0.0 0.0 (* AxisValue (`self.RotationSpeed`)))))

(event `InputAxisKey|MouseY`
  (params (AxisValue :type "Float (single-precision)"))
  ;[1 1 1] Look out
  (`self.K2_AddActorLocalRotation` (`KismetMathLibrary.MakeRotator` 0.0 (* AxisValue (`self.RotationSpeed`)))))

(fn `OnMazeGenerated`
  (`self.K2_SetActorLocation` self (`KismetMathLibrary.MakeVector` (/ (* (`MazeGenerator.Width` (`self.Maze`)) (`MazeGenerator.Step` (`self.Maze`))) 2.0) (/ (* (`MazeGenerator.Height` (`self.Maze`)) (`MazeGenerator.Step` (`self.Maze`))) 2.0) (.z (`self.K2_GetActorLocation` (`self.Maze`)))) false false)
  (set `SpringArmComponent.TargetArmLength` (+ (* (`MazeGenerator.Width` (`self.Maze`)) (`MazeGenerator.Step` (`self.Maze`))) (* (`MazeGenerator.Height` (`self.Maze`)) (`MazeGenerator.Step` (`self.Maze`)))) (`self.SpringArm`))
  (set `self.MinArmLenght` (/ (`SpringArmComponent.TargetArmLength` (`self.SpringArm`)) 3.0)))

(fn `RemoveBalls`
  (bind _outactors (`GameplayStatics.GetAllActorsWithTag` "Ball"))
  (for _array_element _outactors
    (`self.K2_DestroyActor` _array_element)))

(fn `SetStartParams`
  (`Controller.Possess` (`GameplayStatics.GetPlayerController` 0) self)
  (`PlayerController.SetViewTargetWithBlend` (`GameplayStatics.GetPlayerController` 0) self 0.0 "VTBlend_Linear" 0.0 true)
  (set `PlayerController.bShowMouseCursor` true (`GameplayStatics.GetPlayerController` 0))
  (`WidgetBlueprintLibrary.SetInputMode_GameAndUIEx` (`GameplayStatics.GetPlayerController` 0) null)
  (`self.Maze`
    (:`then`
      (`self.OnMazeGenerated`))
    (:`else`)))

(fn `SpawnBall`
  (bind (_hitresult _returnvalue) (`PlayerController.GetHitResultUnderCursorByChannel` (`GameplayStatics.GetPlayerController` 0) "TraceTypeQuery1" true))
  (`self.Maze`
    (:`then`
      (if _returnvalue
        (`|SpawnActorFromClass` "/Game/Blueprints/BP_FallingBall.BP_FallingBall_C" (`KismetMathLibrary.MakeTransform` (`KismetMathLibrary.MakeVector` (.x (`.Location` (`GameplayStatics.BreakHitResult` _hitresult))) (.y (`.Location` (`GameplayStatics.BreakHitResult` _hitresult))) (/ (`SpringArmComponent.TargetArmLength` (`self.SpringArm`)) 3.0))) "AdjustIfPossibleButAlwaysSpawn" "OverrideRootScale" self null)))
    (:`else`)))

(fn `UserConstructionScript`)